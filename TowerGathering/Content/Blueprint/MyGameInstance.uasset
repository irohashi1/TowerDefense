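; Game instance that tracks level transitions and holds the user master data.
; StateLevel records the previous and next level names, starts a fade-out through FadeBP and sets a JumpLevel flag.
; Save copies data into a newly created SaveGameBP, and load reads from a cached or newly created one, with no slot read or write.
; A setter and getter expose the in-memory data.
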(fn StateLevel
  (params (NextLevelName :type Name))
  (Variables|Default|SetOldLevelName (Variables|Default|GetLevelName))
  (Variables|Default|SetLevelName NextLevelName)
  (Default|FadeOutEvent (Variables|Default|GetFadeBP))
  (Variables|Default|SetJumpLevel true))

(fn SaveUserMasterData
  (params (UserMasterData :type User%20Master%20Data%20Structure))
  (bind _returnvalue (SaveGame|CreateSaveGameObject "/Game/Blueprint/SaveGameBP.SaveGameBP_C"))
  (bind _assave_game_bp (Utilities|Casting|CastToSaveGameBP _returnvalue)
    (:then
      (Variables|/Game/Blueprint/SaveGameBP.SaveGameBP_C|SetUserMasterData _assave_game_bp UserMasterData)
      (return true))
    (:CastFailed
      (return false))))

(fn LoadUserMasterData
  (if (== (Variables|Default|GetSaveGameRef) 0)
    (bind _returnvalue (SaveGame|CreateSaveGameObject "/Game/Blueprint/SaveGameBP.SaveGameBP_C"))
    (bind _output_get (Variables|Default|SetSaveGameRef _returnvalue)))
  (bind _assave_game_bp (Utilities|Casting|CastToSaveGameBP _output_get))
  (Variables|Default|SetUserMasterData (Variables|/Game/Blueprint/SaveGameBP.SaveGameBP_C|GetUserMasterData _assave_game_bp)))

(fn SetUserMaster
  (params (data :type User%20Master%20Data%20Structure))
  (Variables|Default|SetUserMasterData data)
  (return))

(fn GetUserMasterData
  (return (Variables|Default|GetUserMasterData)))