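; Auto spawner that releases waves of enemies at random intervals and at random BP_EnemyPos locations.
; On BeginPlay it caches time, enemy and enemy-list DataTable rows plus spawn transforms, then starts a random-delay timer.
; When that fires, it builds SpawnList by comparing each enemy's list ID to a randomly drawn one, re-rolled per enemy.
; A looping one-second timer spawns the list at one position, then schedules the next wave.
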(event EventBeginPlay
  (Utilities|FlowControl|Sequence
    (:then_0
      (CallFunction|GetTimeDatas))
    (:then_1
      (CallFunction|GetEnemyDatas)
      (CallFunction|GetEnemyLists)
      (CallFunction|GetEnemyPos))
    (:then_2
      (CallFunction|SetUpTime))))

(event Collision|EventActorBeginOverlap
  (params (OtherActor :type Actor%20Object%20Reference)))

(event EventTick
  (params (DeltaSeconds :type Float%20%28single-precision%29)))

(fn ConstructionScript)

(fn GetTimeDatas
  (bind _outrownames (DataTable|GetDataTableRowNames "/Game/Blueprint/DataTable/TimeTable.TimeTable"))
  (for (_array_element _array_index) _outrownames
    (bind _returnvalue (Utilities|GetDataTableRow "/Game/Blueprint/DataTable/TimeTable.TimeTable" _array_element)
      (:then
        (Utilities|Array|Insert (Variables|Default|GetTimeTables) _returnvalue _array_index)))))

(fn GetEnemyDatas
  (bind _outrownames (DataTable|GetDataTableRowNames "/Game/Blueprint/DataTable/EnemyTable.EnemyTable"))
  (for (_array_element _array_index) _outrownames
    (bind _returnvalue (Utilities|GetDataTableRow "/Game/Blueprint/DataTable/EnemyTable.EnemyTable" _array_element)
      (:then
        (Utilities|Array|Insert (Variables|Default|GetEnemyTables) _returnvalue _array_index)))))

(fn SetUpTime
  (CallFunction|SetCurrentTime)
  (Utilities|Time|SetTimerbyFunctionName self "AddReservationlist" (Variables|Default|GetCurrentTime)))

(fn AddReservationlist
  (bind _spawnlist (Variables|Default|GetSpawnList))
  (Utilities|Array|Clear (Variables|Default|GetSpawnList))
  (for (_array_element _array_index) (Variables|Default|GetEnemyTables)
    (if (== (.enemylistid _array_element) (.enemylistid (Utilities|Array|Get(acopy) (Variables|Default|GetEnemyListTables) (Math|Random|RandomInteger (Utilities|Array|Length (Variables|Default|GetEnemyListTables))))))
      (Utilities|Array|Insert _spawnlist (Utilities|Array|Get(acopy) (Variables|Default|GetEnemyTables) _array_index) (Utilities|Array|Length _spawnlist))))
  (CallFunction|EnemySpawnRady))

(fn SetCurrentTime
  (Variables|Default|SetCurrentTime (.sec (Utilities|Array|Get(acopy) (Variables|Default|GetTimeTables) (Math|Random|RandomInteger (Utilities|Array|Length (Variables|Default|GetTimeTables)))))))

(fn GetEnemyLists
  (bind _outrownames (DataTable|GetDataTableRowNames "/Game/Blueprint/DataTable/EnemyListTable.EnemyListTable"))
  (for (_array_element _array_index) _outrownames
    (bind _returnvalue (Utilities|GetDataTableRow "/Game/Blueprint/DataTable/EnemyListTable.EnemyListTable" _array_element)
      (:then
        (Utilities|Array|Insert (Variables|Default|GetEnemyListTables) _returnvalue _array_index)))))

(fn EnemySpawn
  (Game|SpawnActorfromClass (.enemyclass (Utilities|Array|Get(acopy) (Variables|Default|GetSpawnList) (Variables|Default|GetCurrentSpawnNum))) (Variables|Default|GetCurrentPos) "Undefined" 0 0)
  (bind _result (Math|Integer|IncrementInt (Variables|Default|GetCurrentSpawnNum))
    (:%20%20
      (if (>= _result (Utilities|Array|Length (Variables|Default|GetSpawnList)))
        (Utilities|Time|ClearandInvalidateTimerbyHandle (Variables|Default|GetSpawnTimeHandler))
        (CallFunction|SetUpTime)))))

(fn EnemySpawnRady
  (CallFunction|SetPosNum)
  (Variables|Default|SetCurrentSpawnNum 0)
  (bind _returnvalue (Utilities|Time|SetTimerbyFunctionName self "EnemySpawn" 1.0 true))
  (Variables|Default|SetSpawnTimeHandler _returnvalue))

(fn GetEnemyPos
  (bind _outactors (Actor|GetAllActorsOfClass "/Game/Blueprint/object/BP_EnemyPos.BP_EnemyPos_C"))
  (for (_array_element _array_index) _outactors
    (Utilities|Array|Insert (Variables|Default|GetPosList) (Transformation|GetActorTransform _array_element) _array_index)))

(fn SetPosNum
  (Variables|Default|SetCurrentPos (Utilities|Array|Get(acopy) (Variables|Default|GetPosList) (Math|Random|RandomInteger (Utilities|Array|Length (Variables|Default|GetPosList))))))