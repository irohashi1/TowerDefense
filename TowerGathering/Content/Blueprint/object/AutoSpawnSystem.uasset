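; AutoSpawnSystem is an actor that loads data tables, apparently for automatic enemy spawning.
; On BeginPlay, GetTimeDatas and GetEnemyDatas walk every row name of TimeTable and EnemyListTable.
; Each found row is inserted at its loop index into the TimeTables and EnemyTables arrays.
; The graphs contain no spawn logic, and Tick and overlap events are empty.
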(event EventBeginPlay
  (CallFunction|GetTimeDatas)
  (CallFunction|GetEnemyDatas))

(event Collision|EventActorBeginOverlap
  (params (OtherActor :type Actor%20Object%20Reference)))

(event EventTick
  (params (DeltaSeconds :type Float%20%28single-precision%29)))

(fn ConstructionScript)

(fn GetTimeDatas
  (bind _outrownames (DataTable|GetDataTableRowNames "/Game/Blueprint/DataTable/TimeTable.TimeTable"))
  (for (_array_element _array_index) _outrownames
    (bind _returnvalue (Utilities|GetDataTableRow "/Game/Blueprint/DataTable/TimeTable.TimeTable" _array_element)
      (:then
        (Utilities|Array|Insert (Variables|Default|GetTimeTables) _returnvalue _array_index)))))

(fn GetEnemyDatas
  (bind _outrownames (DataTable|GetDataTableRowNames "/Game/Blueprint/DataTable/EnemyListTable.EnemyListTable"))
  (for (_array_element _array_index) _outrownames
    (bind _returnvalue (Utilities|GetDataTableRow "/Game/Blueprint/DataTable/EnemyListTable.EnemyListTable" _array_element)
      (:then
        (Utilities|Array|Insert (Variables|Default|GetEnemyTables) _returnvalue _array_index)))))