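; Bird's-eye camera Blueprint that handles mouse-driven camera control and click selection of BP_Servant actors.
; Right-drag adds controller yaw and pitch, while middle-drag pans and the wheel dollies through local-space movement scaled by ZoomForce.
; Releasing left click traces from the deprojected cursor on the Camera channel.
; A servant hit passes its name and Param to a lazily created, reused WD_ObjectStatus widget.
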(event EventBeginPlay)

(event Collision|EventActorBeginOverlap
  (params (OtherActor :type Actor%20Object%20Reference)))

(event EventTick
  (params (DeltaSeconds :type Float%20%28single-precision%29)))

(event Input|ActionEvents|InputActionCenterClick
  (params (Key :type Key%20Structure :default "AnyKey"))
  ;[1 1 1] Camera Input Flg
  (:Pressed
    (Variables|Default|SetIsCameraInputMove true))
  (:Released
    (Variables|Default|SetIsCameraInputMove false)))

(event Input|ActionEvents|InputActionLeftClick
  (params (Key :type Key%20Structure :default "AnyKey"))
  (:Released
    (bind _ishit (CallFunction|HitCheck))
    (if _ishit
      (CallFunction|SwitchHitProc))))

(event Input|ActionEvents|InputActionRightClick
  (params (Key :type Key%20Structure :default "AnyKey"))
  ;[1 1 1] Camera Input Flg
  (:Pressed
    (Variables|Default|SetIsCameraInputRotate true))
  (:Released
    (Variables|Default|SetIsCameraInputRotate false)))

(event Input|AxisEvents|InputAxisTurn
  (params (AxisValue :type Float%20%28single-precision%29))
  ;[1 1 1] Input
  ;[1 1 1] Camera Rotate
  (if (Variables|Default|GetIsCameraInputRotate)
    (Pawn|Input|AddControllerYawInput AxisValue)
    (else
      ;[1 1 1] Camera Move
      (if (Variables|Default|GetIsCameraInputMove)
        (CallFunction|InputCameraMove (Math|Vector|MakeVector 0.0 AxisValue 0.0))))))

(event Input|AxisEvents|InputAxisLookUp
  (params (AxisValue :type Float%20%28single-precision%29))
  ;[1 1 1] Input
  ;[1 1 1] Camera Rotate
  (if (Variables|Default|GetIsCameraInputRotate)
    (Pawn|Input|AddControllerPitchInput AxisValue)
    (else
      ;[1 1 1] Camera Move
      (if (Variables|Default|GetIsCameraInputMove)
        (CallFunction|InputCameraMove (Math|Vector|MakeVector 0.0 0.0 AxisValue))))))

(event Input|MouseEvents|MouseWheelAxis
  (params (AxisValue :type Float%20%28single-precision%29))
  ;[1 1 1] Input
  ;[1 1 1] Camera Move
  (CallFunction|InputCameraMove (Math|Vector|MakeVector AxisValue 0.0 0.0)))

(fn ConstructionScript)

(fn HitCheck
  (bind _returnvalue (Game|GetPlayerController 0))
  (bind (_worldlocation _worlddirection) (Game|Player|ConvertMouseLocationToWorldSpace _returnvalue))
  (bind (_outhit _returnvalue_2) (Collision|LineTraceByChannel _worldlocation (+ _worldlocation (* _worlddirection 1000000)) "TraceTypeQuery2" false 0 "None"))
  (Variables|Default|SetHitData _outhit)
  (return _returnvalue_2))

(fn SettingCamera)

(fn InputCameraMove
  (params (Move :type Vector))
  (Class|Actor|AddActorLocalTransform (Math|Transform|MakeTransform (* Move (Variables|Default|GetZoomForce)) "0, 0, 0" "1,1,1") false false))

(fn InputCameraRotate
  (params (Move :type Rotator)))

(fn SwitchHitProc
  (bind _asbp_servant (Utilities|Casting|CastToBP_Servant (.HitActor (Collision|BreakHitResult (Variables|Default|GetHitData)))))
  (CallFunction|SetObjectStatusRef (Variables|/Game/BluePrint/object/BP_Character.BP_Character_C|Getparam _asbp_servant) _asbp_servant))

(fn SetObjectStatusRef
  (params (Param :type Character%20Parameter%20Structure) (TargetRef :type Actor%20Object%20Reference))
  (if (Utilities|IsValid (Variables|Default|GetObjectStatusRef))
    _
    (else
      (bind _returnvalue (UserInterface|CreateWidget "/Game/Blueprint/Widget/WD_ObjectStatus.WD_ObjectStatus_C"))
      (UserInterface|Viewport|AddtoViewport _returnvalue 0)
      (Variables|Default|SetObjectStatusRef _returnvalue)))
  (Variables|/Game/Blueprint/Widget/WD_ObjectStatus.WD_ObjectStatus_C|SetTargetName (Variables|Default|GetObjectStatusRef) (Utilities|GetObjectName TargetRef))
  (Variables|/Game/Blueprint/Widget/WD_ObjectStatus.WD_ObjectStatus_C|SetParameter (Variables|Default|GetObjectStatusRef) Param))