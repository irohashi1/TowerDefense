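; Save game Blueprint that stores user master data as a list of slots with the newest entry first.
; New inserts an entry at the front and trims the list to five.
; Save inserts at the front, then removes the given index, which applies to the already shifted list, and resets that index to zero.
; Load returns one entry by index and LoadAll returns the whole list.
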(fn Save
  (params (data :type User%20Master%20Data%20Structure) (Num :type Integer%20%28by%20ref%29))
  (Utilities|Array|Insert (Variables|Default|GetUserMasterData) data)
  (Utilities|Array|RemoveIndex (Variables|Default|GetUserMasterData) Num)
  (|SetBy-RefVar Num 0))

(fn Load
  (params (Num :type Integer))
  (return (Utilities|Array|Get(acopy) (Variables|Default|GetUserMasterData) Num)))

(fn New
  (params (data :type User%20Master%20Data%20Structure))
  (bind _usermasterdata (Variables|Default|GetUserMasterData))
  (Utilities|Array|Insert _usermasterdata data)
  (if (> (Utilities|Array|Length _usermasterdata) 5)
    (Utilities|Array|Resize (Variables|Default|GetUserMasterData) 5)))

(fn LoadAll
  (return (Variables|Default|GetUserMasterData)))