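; BP_MouseAction is an actor that spawns test cubes where the player clicks in the world.
; On left mouse release it deprojects the cursor and runs a 3000-unit Visibility line trace along that ray.
; A hit spawns a BP_TestCube at the hit location, while a miss prints a message.
; The press event only prints a debug string.
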(event EventBeginPlay)

(event Collision|EventActorBeginOverlap
  (params (OtherActor :type Actor%20Object%20Reference)))

(event EventTick
  (params (DeltaSeconds :type Float%20%28single-precision%29)))

(event Input|MouseEvents|LeftMouseButton
  (params (Key :type Key%20Structure :default "AnyKey"))
  (bind _returnvalue (Game|GetPlayerController 0))
  (bind (_worldlocation _worlddirection) (Game|Player|ConvertMouseLocationToWorldSpace _returnvalue))
  (:Pressed
    (Development|PrintString "Pressed"))
  (:Released
    (bind (_outhit _returnvalue_2) (Collision|LineTraceByChannel _worldlocation (+ _worldlocation (* _worlddirection 3000)) "TraceTypeQuery1" false 0 "None"))
    (if _returnvalue_2
      (Game|SpawnActorfromClass "/Game/Blueprint/BP_TestCube.BP_TestCube_C" (Math|Conversions|ToTransform(Vector) (.Location (Collision|BreakHitResult _outhit))) "Undefined" 0 0)
      (else
        (Development|PrintString "No hit")))))

(fn ConstructionScript)