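; Game instance that holds user master data and level-change state for the game.
; StateLevel records the old and next level names, triggers the FadeBP fade-out and sets JumpLevel, without opening the level itself.
; Getters and setters expose UserMasterData, while save and load copy it through BP_SaveGame objects created in memory, with no slot reads or writes.
; A small function wraps showing the mouse cursor.
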(fn StateLevel
  (params (NextLevelName :type Name))
  (Variables|Default|SetOldLevelName (Variables|Default|GetLevelName))
  (Variables|Default|SetLevelName NextLevelName)
  (Default|FadeOutEvent (Variables|Default|GetFadeBP))
  (Variables|Default|SetJumpLevel true))

(fn SaveUserMasterData
  (params (UserMasterData :type User%20Master%20Data%20Structure))
  (bind _returnvalue (SaveGame|CreateSaveGameObject "/Game/Blueprint/BP_SaveGame.BP_SaveGame_C"))
  (bind _asbp_save_game (Utilities|Casting|CastToBP_SaveGame _returnvalue)
    (:then
      (Variables|/Game/Blueprint/BP_SaveGame.BP_SaveGame_C|SetUserMasterData _asbp_save_game UserMasterData)
      (return true))
    (:CastFailed
      (return false))))

(fn LoadUserMasterData
  (if (== (Variables|Default|GetSaveGameRef) 0)
    (bind _returnvalue (SaveGame|CreateSaveGameObject "/Game/Blueprint/BP_SaveGame.BP_SaveGame_C"))
    (bind _output_get (Variables|Default|SetSaveGameRef _returnvalue)))
  (bind _asbp_save_game (Utilities|Casting|CastToBP_SaveGame _output_get))
  (Variables|Default|SetUserMasterData (Variables|/Game/Blueprint/BP_SaveGame.BP_SaveGame_C|GetUserMasterData _asbp_save_game)))

(fn SetUserMaster
  (params (data :type User%20Master%20Data%20Structure))
  (Variables|Default|SetUserMasterData data)
  (return))

(fn GetUserMasterData
  (return (Variables|Default|GetUserMasterData)))

(fn ShowMouseCursor
  (CallFunction|ShowMouseCursor))