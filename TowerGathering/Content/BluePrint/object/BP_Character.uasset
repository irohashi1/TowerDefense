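; BP_Character is a combat character base that manages attack, damage and death states.
; Start functions set movement and action flags, then call empty Begin hooks; damage subtracts hit points and routes to death at zero or below, disabling capsule collision.
; AttackHitBegin selects parameters by attack type, then positions, scales and enables a reusable sphere or box hitbox, which AttackHitEnd collapses and disables.
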(fn ConstructionScript)

(fn AttackStart
  (Variables|Default|SetAttacking true)
  (Variables|Default|SetCanWalk false)
  (CallFunction|AttackBegin))

(fn AttackEnd
  (Variables|Default|SetCanWalk true)
  (Variables|Default|SetAttacking false))

(fn AttackBegin)

(fn DamageStart
  (params (DamagePoint :type Integer))
  (bind _output_get (Variables|Default|Setparam (Utilities|Struct|MakeCharacterParameter (- (.HitPoint (Utilities|Struct|BreakCharacterParameter (Variables|Default|Getparam))) DamagePoint) (.Speed (Utilities|Struct|BreakCharacterParameter (Variables|Default|Getparam))) (.AttackPoint (Utilities|Struct|BreakCharacterParameter (Variables|Default|Getparam))) (.DefensePoint (Utilities|Struct|BreakCharacterParameter (Variables|Default|Getparam))) (.Type (Utilities|Struct|BreakCharacterParameter (Variables|Default|Getparam))))))
  (Variables|Default|SetAttacking false)
  (Variables|Default|SetSteped false)
  (Variables|Default|SetCanWalk false)
  (if (> (.HitPoint (Utilities|Struct|BreakCharacterParameter _output_get)) 0)
    (CallFunction|DamageBegin)
    (else
      (CallFunction|DeathStart))))

(fn DamageEnd
  (Variables|Default|SetCanWalk true))

(fn DamageBegin)

(fn DeathStart
  (Collision|SetCollisionEnabled (Variables|Collision|GetCapsuleComponent) "NoCollision")
  (CallFunction|DeathBegin))

(fn DeathEnd)

(fn DeathBegin)

(fn AttackHitBegin
  (params (AttackType :type AttackType%20Enum))
  (bind _sphere (Variables|Default|GetSphere))
  (bind _box (Variables|Default|GetBox))
  (switch Utilities|FlowControl|Switch|SwitchonAttackType AttackType
    (:NewEnumerator0
      (LocalVariables|SetAttack_Param (Variables|Default|GetAttackA_Param)))
    (:NewEnumerator1
      (LocalVariables|SetAttack_Param (Variables|Default|GetAttackB_Param)))
    (:NewEnumerator2
      (LocalVariables|SetAttack_Param (Variables|Default|GetAttackA_Heavy_Param)))
    (:NewEnumerator3
      (LocalVariables|SetAttack_Param (Variables|Default|GetAttackB_Heavy_Param))))
  (switch Utilities|FlowControl|Switch|SwitchonAttackRangeType (.RangeType (Utilities|Struct|BreakAttackParameter (LocalVariables|GetAttack_Param)))
    (:NewEnumerator0
      (Transformation|SetRelativeLocation _sphere (.Offset (Utilities|Struct|BreakAttackParameter (LocalVariables|GetAttack_Param))) false true)
      (Transformation|SetWorldScale3D _sphere (.Range (Utilities|Struct|BreakAttackParameter (LocalVariables|GetAttack_Param))))
      (Collision|SetCollisionEnabled _sphere "QueryAndPhysics"))
    (:NewEnumerator1
      (Transformation|SetRelativeLocation _box (.Offset (Utilities|Struct|BreakAttackParameter (LocalVariables|GetAttack_Param))) false true)
      (Transformation|SetWorldScale3D _box (.Range (Utilities|Struct|BreakAttackParameter (LocalVariables|GetAttack_Param))))
      (Collision|SetCollisionEnabled _box "QueryAndPhysics"))))

(fn AttackHitEnd
  (params (AttackType :type AttackType%20Enum))
  (bind _sphere (Variables|Default|GetSphere))
  (bind _box (Variables|Default|GetBox))
  (switch Utilities|FlowControl|Switch|SwitchonAttackType AttackType
    (:NewEnumerator0
      (LocalVariables|SetAttack_Param (Variables|Default|GetAttackA_Param)))
    (:NewEnumerator1
      (LocalVariables|SetAttack_Param (Variables|Default|GetAttackB_Param)))
    (:NewEnumerator2
      (LocalVariables|SetAttack_Param (Variables|Default|GetAttackA_Heavy_Param)))
    (:NewEnumerator3
      (LocalVariables|SetAttack_Param (Variables|Default|GetAttackB_Heavy_Param))))
  (switch Utilities|FlowControl|Switch|SwitchonAttackRangeType (.RangeType (Utilities|Struct|BreakAttackParameter (LocalVariables|GetAttack_Param)))
    (:NewEnumerator0
      (Transformation|SetRelativeLocation _sphere "0, 0, 0" false true)
      (Transformation|SetWorldScale3D _sphere "0, 0, 0")
      (Collision|SetCollisionEnabled _sphere "NoCollision"))
    (:NewEnumerator1
      (Transformation|SetRelativeLocation _box "0, 0, 0" false true)
      (Transformation|SetWorldScale3D _box "0, 0, 0")
      (Collision|SetCollisionEnabled _box "NoCollision"))))