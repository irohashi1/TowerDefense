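; BP_Charcter is a base character Blueprint that manages attack, damage and death states for game characters.
; Start functions set the Attacking, Steped and CanWalk flags, then call empty Begin hooks, apparently for child classes to override.
; DamageStart subtracts damage from the HitPoint field in the Param struct, then branches to DamageBegin or DeathStart.
; AttackEnd and DamageEnd restore walking, while DeathEnd is empty.
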(fn ConstructionScript)

(fn AttackStart
  (Variables|Default|SetAttacking true)
  (Variables|Default|SetCanWalk false)
  (CallFunction|AttackBegin))

(fn AttackEnd
  (Variables|Default|SetCanWalk true)
  (Variables|Default|SetAttacking false))

(fn AttackBegin)

(fn DamageStart
  (params (DamagePoint :type Integer))
  (bind _output_get (Variables|Default|Setparam (Utilities|Struct|MakeCharacterParameter (- (.HitPoint (Utilities|Struct|BreakCharacterParameter (Variables|Default|Getparam))) DamagePoint) (.Speed (Utilities|Struct|BreakCharacterParameter (Variables|Default|Getparam))) (.AttackPoint (Utilities|Struct|BreakCharacterParameter (Variables|Default|Getparam))) (.DefensePoint (Utilities|Struct|BreakCharacterParameter (Variables|Default|Getparam))) (.Type (Utilities|Struct|BreakCharacterParameter (Variables|Default|Getparam))))))
  (Variables|Default|SetAttacking false)
  (Variables|Default|SetSteped false)
  (Variables|Default|SetCanWalk false)
  (if (> (.HitPoint (Utilities|Struct|BreakCharacterParameter _output_get)) 0)
    (CallFunction|DamageBegin)
    (else
      (CallFunction|DeathStart))))

(fn DamageEnd
  (Variables|Default|SetCanWalk true))

(fn DamageBegin)

(fn DeathStart
  (CallFunction|DeathBegin))

(fn DeathEnd)

(fn DeathBegin)