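; BP_Servant is a player-controllable servant character with movement, camera look and attacking.
; Axis inputs drive control rotation and yaw-relative movement, gated by CanWalk and scaled by Param.Speed, while the Attack action calls AttackStart.
; Box and Sphere overlaps act as hitboxes, passing truncated Param.AttackPoint to DamageStart on other BP_Character actors.
; Space bar applies hardcoded damage to the servant itself.
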(event OnComponentBeginOverlap(Box)
  (params (OverlappedComponent :type Primitive%20Component%20Object%20Reference) (OtherActor :type Actor%20Object%20Reference) (OtherComp :type Primitive%20Component%20Object%20Reference) (OtherBodyIndex :type Integer) (bFromSweep :type Boolean) (SweepResult :type Hit%20Result%20Structure%20%28by%20ref%29))
  (if (!= (Class|PawnMovementComponent|GetPawnOwner (Variables|Character|GetCharacterMovement)) OtherActor)
    (bind _asbp_character (Utilities|Casting|CastToBP_Character OtherActor))
    (Default|DamageStart _asbp_character (Math|Float|Truncate (.AttackPoint (Utilities|Struct|BreakCharacterParameter (Variables|Default|Getparam)))))))

(event OnComponentBeginOverlap(Sphere)
  (params (OverlappedComponent :type Primitive%20Component%20Object%20Reference) (OtherActor :type Actor%20Object%20Reference) (OtherComp :type Primitive%20Component%20Object%20Reference) (OtherBodyIndex :type Integer) (bFromSweep :type Boolean) (SweepResult :type Hit%20Result%20Structure%20%28by%20ref%29))
  (if (!= (Class|PawnMovementComponent|GetPawnOwner (Variables|Character|GetCharacterMovement)) OtherActor)
    (bind _asbp_character (Utilities|Casting|CastToBP_Character OtherActor))
    (Default|DamageStart _asbp_character (Math|Float|Truncate (.AttackPoint (Utilities|Struct|BreakCharacterParameter (Variables|Default|Getparam)))))))

(event Input|ActionEvents|InputActionAttack
  (params (Key :type Key%20Structure :default "AnyKey"))
  (:Pressed
    (CallFunction|AttackStart)))

(event Input|AxisEvents|InputAxisTurn
  (params (AxisValue :type Float%20%28single-precision%29))
  ;[1 1 1] Move
  (Pawn|Input|AddControllerYawInput AxisValue))

(event Input|AxisEvents|InputAxisMoveRight
  (params (AxisValue :type Float%20%28single-precision%29))
  ;[1 1 1] Move
  (if (Variables|Default|GetCanWalk)
    (Pawn|Input|AddMovementInput (Math|Vector|GetRightVector (Math|Rotator|MakeRotator 0.0 0.0 (.Yaw (Math|Rotator|BreakRotator (Pawn|GetControlRotation :!class /Script/Engine.Pawn))))) (* AxisValue (.Speed (Utilities|Struct|BreakCharacterParameter (Variables|Default|Getparam)))) false)))

(event Input|AxisEvents|InputAxisLookUp
  (params (AxisValue :type Float%20%28single-precision%29))
  ;[1 1 1] Move
  (Pawn|Input|AddControllerPitchInput AxisValue))

(event Input|AxisEvents|InputAxisMoveFoward
  (params (AxisValue :type Float%20%28single-precision%29))
  ;[1 1 1] Move
  (if (Variables|Default|GetCanWalk)
    (Pawn|Input|AddMovementInput (Math|Vector|GetForwardVector (Math|Rotator|MakeRotator 0.0 0.0 (.Yaw (Math|Rotator|BreakRotator (Pawn|GetControlRotation :!class /Script/Engine.Pawn))))) (* AxisValue (.Speed (Utilities|Struct|BreakCharacterParameter (Variables|Default|Getparam)))) false)))

(event Input|KeyboardEvents|SpaceBar
  (params (Key :type Key%20Structure :default "AnyKey"))
  (:Pressed
    (CallFunction|DamageStart 500)))

(fn ConstructionScript
  (|CallParentFunction))