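; BP_PlayerBase is the player's base, with hit points that can be damaged and recovered.
; On BeginPlay it fills Hp to MaxHp and registers itself with BP_GM_Main as PlayerBase.
; Damage subtracts from Hp and, at zero or below, has BP_MyGameInstance switch to the result level.
; Recovery adds points, capped at MaxHp.
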(event EventBeginPlay
  (Variables|Default|SetHp (Variables|Default|GetMaxHp))
  (bind _asbp_gm_main (Utilities|Casting|CastToBP_GM_Main (Game|GetGameMode)))
  (Variables|/Game/BluePrint/BP_GM_Main.BP_GM_Main_C|SetPlayerBase _asbp_gm_main self))

(event Collision|EventActorBeginOverlap
  (params (OtherActor :type Actor%20Object%20Reference)))

(event EventTick
  (params (DeltaSeconds :type Float%20%28single-precision%29)))

(fn ConstructionScript)

(fn Damage
  (params (point :type Integer))
  (Variables|Default|SetHp (- (Variables|Default|GetHp) point))
  (if (<= (Variables|Default|GetHp) 0)
    (CallFunction|StateLevel)))

(fn Recovery
  (params (Point :type Integer))
  (bind _maxhp (Variables|Default|GetMaxHp))
  (Variables|Default|SetHp (Math|Integer|SelectInt (+ Point (Variables|Default|GetHp)) _maxhp (< (+ Point (Variables|Default|GetHp)) _maxhp))))

(fn StateLevel
  (bind _asbp_my_game_instance (Utilities|Casting|CastToBP_MyGameInstance (Game|GetGameInstance)))
  (Default|StateLevel _asbp_my_game_instance "L_result"))