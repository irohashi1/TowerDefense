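; BP_GM_Main, apparently the main game mode, tracks allied servants and enemies in two lists.
; On registration, each unit receives both lists and the player base through SetFieldInfo; enemies are also flagged as Enemy.
; SpawnEnemy creates a troll servant with the enemy behavior tree, assigns the enemy AI controller class after spawning, and registers it as an enemy.
; BeginPlay, Tick and the construction script are empty.
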(event EventBeginPlay)

(event EventTick
  (params (DeltaSeconds :type Float%20%28single-precision%29)))

(fn ConstructionScript)

(fn AddServantList
  (params (Servant :type BP%20Servant%20Object%20Reference))
  (Default|SetFieldInfo Servant (Variables|Default|GetServantList) (Variables|Default|GetEnemyList) (Variables|Default|GetPlayerBase))
  (Utilities|Array|Add (Variables|Default|GetServantList) Servant))

(fn RemoveServantList
  (params (Servant :type BP%20Servant%20Object%20Reference))
  (Utilities|Array|RemoveItem (Variables|Default|GetServantList) Servant))

(fn AddEnemyList
  (params (Enemy :type BP%20Servant%20Object%20Reference))
  (Variables|/Game/BluePrint/object/Servant/BP_Servant.BP_Servant_C|SetEnemy Enemy true)
  (Default|SetFieldInfo Enemy (Variables|Default|GetServantList) (Variables|Default|GetEnemyList) (Variables|Default|GetPlayerBase))
  (Utilities|Array|Add (Variables|Default|GetEnemyList) Enemy))

(fn RemoveEnemyList
  (params (Enemy :type BP%20Servant%20Object%20Reference))
  (Utilities|Array|RemoveItem (Variables|Default|GetEnemyList) Enemy))

(fn SpawnEnemy
  (params (Location :type Vector) (Rotation :type Rotator))
  (bind _returnvalue (AI|SpawnAIFromClass "/Game/BluePrint/object/Servant/Giant/BP_Servant_Troll.BP_Servant_Troll_C" "/Game/BluePrint/AI/Enemy/BT_Enemy.BT_Enemy" Location Rotation false))
  (Variables|/Script/Engine.Pawn|SetAIControllerClass _returnvalue "/Game/BluePrint/AI/Enemy/BP_AI_Enemy.BP_AI_Enemy_C")
  (bind _asbp_servant (Utilities|Casting|CastToBP_Servant _returnvalue))
  (CallFunction|AddEnemyList _asbp_servant))